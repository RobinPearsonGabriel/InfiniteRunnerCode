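; Runner character Blueprint that adds a death effect on top of its parent class.
; BeginPlay, ActorBeginOverlap and Tick only forward to the parent.
; On Die it calls the parent, hides the mesh without affecting its children, then spawns an explosion particle and plays an explosion sound at the mesh's world location.
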(event EventBeginPlay
  (|CallParentFunction))

(event Collision|EventActorBeginOverlap
  (params (OtherActor :type Actor%20Object%20Reference))
  (|CallParentFunction OtherActor))

(event EventTick
  (params (DeltaSeconds :type Float%20%28single-precision%29))
  (|CallParentFunction DeltaSeconds))

(event EventDie
  (bind _self self)
  (bind _mesh (Variables|Character|GetMesh _self))
  (bind _returnvalue (Transformation|GetWorldLocation _mesh))
  (|CallParentFunction)
  (Rendering|SetVisibility (Variables|Character|GetMesh) false false)
  (Effects|SpawnEmitteratLocation "/Game/StarterContent/Particles/P_Explosion.P_Explosion" _returnvalue)
  (Audio|PlaySoundatLocation "/Game/StarterContent/Audio/Explosion01.Explosion01" _returnvalue "0, 0, 0" 1.0 1.0 0.0 0 0 0))

(fn ConstructionScript)